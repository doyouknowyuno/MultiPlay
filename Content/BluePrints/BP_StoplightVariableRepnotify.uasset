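; Stoplight actor that demonstrates RepNotify variables by cycling a traffic light through blinking, green, yellow and red.
; On BeginPlay only the authority runs an endless Delay-driven loop that sets the StreetlightScalar and BlinkScalar variables.
; Their OnRep functions push each value into a dynamic material instance, created on the traffic light mesh in the construction script, so the visuals follow the replicated state.
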(event EventBeginPlay
  (Networking|SwitchHasAuthority :!label _label
    (:Authority
      (Utilities|FlowControl|Delay 0.2)
      (Variables|Default|SetBlinkScalar (Variables|Default|GetBlinkOff))
      (Utilities|FlowControl|Delay 0.3)
      (Variables|Default|SetBlinkScalar (Variables|Default|GetBlinkOn))
      (Utilities|FlowControl|Delay 0.3)
      (Variables|Default|SetBlinkScalar (Variables|Default|GetBlinkOff))
      (Utilities|FlowControl|Delay 0.3)
      (Variables|Default|SetBlinkScalar (Variables|Default|GetBlinkOn))
      (Utilities|FlowControl|Delay 0.3)
      (Variables|Default|SetBlinkScalar (Variables|Default|GetBlinkOff))
      (Variables|Default|Set%20StreetlightScalar (Variables|Default|Get%20GreenScalar))
      (Utilities|FlowControl|Delay 1.0)
      (Variables|Default|Set%20StreetlightScalar (Variables|Default|GetYellowScalar))
      (Utilities|FlowControl|Delay 1.0)
      (Variables|Default|Set%20StreetlightScalar (Variables|Default|Get%20RedScalar))
      (goto _label))))

(fn ConstructionScript
  (bind _returnvalue (Rendering|Material|CreateDynamicMaterialInstance (Variables|Default|GetSM_Traffic_Light) 1 0 "None" :!class /Script/Engine.PrimitiveComponent))
  (Variables|Default|SetStreetlightMID _returnvalue))

(fn OnRepStreetlightScalar
  (Rendering|Material|SetScalarParameterValue (Variables|Default|GetStreetlightMID) (Variables|Default|Get%20StreetlightScalarParamName) (Variables|Default|Get%20StreetlightScalar) :!class /Script/Engine.MaterialInstanceDynamic))

(fn OnRepBlinkScalar
  (Rendering|Material|SetScalarParameterValue (Variables|Default|GetStreetlightMID) (Variables|Default|GetBlinkParamName) (Variables|Default|GetBlinkScalar) :!class /Script/Engine.MaterialInstanceDynamic))