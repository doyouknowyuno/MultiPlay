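; BP_Variable_Replication_None is an actor that shows a cycling Health value as text, apparently a demo of an unreplicated variable, going by its name.
; On BeginPlay, only the authority calls UpdateHealth and starts a looping timer at the decrement interval.
; UpdateHealth lowers Health and resets it to MaxHealth at zero or below.
; Tick writes the local Health value to the TextRender without an authority check.
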(event EventBeginPlay
  ;[1 1 1] 서버라면/아니면
  (Networking|SwitchHasAuthority
    (:Authority
      (CallFunction|UpdateHealth)
      (Utilities|Time|SetTimerbyFunctionName 0 "" (Variables|Default|GetHealthDecrementTime) true))))

(event Collision|EventActorBeginOverlap
  (params (OtherActor :type Actor%20Object%20Reference)))

(event EventTick
  (params (DeltaSeconds :type Float%20%28single-precision%29))
  (bind _textrender (Variables|Default|GetTextRender))
  (Utilities|IsValid _textrender
    (:Is%20Valid
      (Rendering|Components|TextRender|SetText _textrender (Utilities|Text|ToText(String) (Utilities|String|BuildString(Integer) "" "Health :" (Variables|Default|GetHealth)))))))

(fn ConstructionScript)

(fn UpdateHealth
  (bind _output_get (Variables|Default|SetHealth (- (Variables|Default|GetHealth) (Variables|Default|GetHealthDecrementAmt))))
  (if (<= _output_get 0)
    (CallFunction|InitializeHealth)))

(fn InitializeHealth
  (Variables|Default|SetHealth (Variables|Default|GetMaxHealth)))