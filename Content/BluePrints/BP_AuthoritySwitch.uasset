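; BP_AuthoritySwitch is an actor that visually shows whether the local instance has network authority.
; On BeginPlay, a Switch Has Authority node sets the text render to either the server or client value.
; Each branch also creates a dynamic M_Ghost_Body material on the ghost mesh and tints its Upper Color blue for authority or pinkish red for remote.
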(event EventBeginPlay
  (Networking|SwitchHasAuthority
    (:Authority
      (Rendering|Components|TextRender|SetText (Variables|Default|GetTextRender) (Variables|Default|GetServerValue))
      (bind _returnvalue (Rendering|Material|CreateDynamicMaterialInstance (Variables|Default|GetSM_Ghost) 0 "/Game/ExampleContent/NetworkFeatures/Materials/M_Ghost_Body.M_Ghost_Body" "None" :!class /Script/Engine.PrimitiveComponent))
      (Rendering|Material|SetVectorParameterValue _returnvalue "Upper Color" "(R=0.080375,G=0.000000,B=1.000000,A=1.000000)" :!class /Script/Engine.MaterialInstanceDynamic))
    (:Remote
      (Rendering|Components|TextRender|SetText (Variables|Default|GetTextRender) (Variables|Default|GetClientValue))
      (bind _returnvalue_2 (Rendering|Material|CreateDynamicMaterialInstance (Variables|Default|GetSM_Ghost) 0 "/Game/ExampleContent/NetworkFeatures/Materials/M_Ghost_Body.M_Ghost_Body" "None" :!class /Script/Engine.PrimitiveComponent))
      (Rendering|Material|SetVectorParameterValue _returnvalue_2 "Upper Color" "(R=1.000000,G=0.000000,B=0.250507,A=1.000000)" :!class /Script/Engine.MaterialInstanceDynamic))))

(fn ConstructionScript)